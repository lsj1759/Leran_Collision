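; BP_ChangeColor is an actor in a collision-learning folder whose cube toggles between red and blue when the player character class BP_MyCharacter begins overlapping it.
; Each overlap switches on the EnumColor state, swaps the cube's material to a vertex color view mode material and flips the enum.
; It then fires a change-color event dispatcher with the new color so bound listeners can react.
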(event OnComponentBeginOverlap(Cube)
  (params (OverlappedComponent :type Primitive%20Component%20Object%20Reference) (OtherActor :type Actor%20Object%20Reference) (OtherComp :type Primitive%20Component%20Object%20Reference) (OtherBodyIndex :type Integer) (bFromSweep :type Boolean) (SweepResult :type Hit%20Result%20Structure%20%28by%20ref%29))
  (Utilities|Casting|CastToBP_MyCharacter OtherActor)
  (switch Utilities|FlowControl|Switch|SwitchonEnum_Color (Variables|Default|GetEnumColor)
    (:NewEnumerator0
      (Rendering|Material|SetMaterial (Variables|Default|GetCube) 0 "/Engine/EngineDebugMaterials/VertexColorViewMode_BlueOnly.VertexColorViewMode_BlueOnly")
      (bind _output_get (Variables|Default|SetEnumColor "NewEnumerator1"))
      (Default|CallEventDispatcherChangeColor _output_get))
    (:NewEnumerator1
      (Rendering|Material|SetMaterial (Variables|Default|GetCube) 0 "/Engine/EngineDebugMaterials/VertexColorViewMode_RedOnly.VertexColorViewMode_RedOnly")
      (bind _output_get_2 (Variables|Default|SetEnumColor "NewEnumerator0"))
      (Default|CallEventDispatcherChangeColor _output_get_2))))

(fn ConstructionScript)
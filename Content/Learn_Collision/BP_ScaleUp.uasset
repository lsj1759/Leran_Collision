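; BP_ScaleUp is a collision-learning actor that enlarges its Cube once every coin in its Coin array is hidden.
; On BeginPlay it binds an event to each coin's hidden-state dispatcher.
; OnHiddenCheck uses CheckCoin to test all coins, then triples the cube's relative scale or resets it to normal.
; A leftover scale node in the event graph never runs.
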(event EventBeginPlay
  (for _array_element (Variables|Default|GetCoin)
    (EventDispatchers|BindEventtoEventDispatcherHidden _array_element (EventDispatchers|CreateEvent :!event OnHiddenCheck))))

(fn ConstructionScript)

(fn OnHiddenCheck
  (bind _isallhidden (CallFunction|CheckCoin))
  (if _isallhidden
    (Transformation|SetRelativeScale3D (Variables|Default|GetCube) "3.000000,3.000000,3.000000")
    (else
      (Transformation|SetRelativeScale3D (Variables|Default|GetCube) "1.000000,1.000000,1.000000"))))

(fn CheckCoin
  (for _array_element (Variables|Default|GetCoin)
    (if (not (Variables|/Script/Engine.Actor|GetbHidden _array_element))
      (return false)))
  (return true))
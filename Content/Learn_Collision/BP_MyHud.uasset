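; BP_MyHud is a HUD Blueprint in the Learn_Collision folder that shows text on screen through a widget.
; On BeginPlay it creates the HUD widget, stores a reference to it and adds it to the viewport.
; SetText and SetLeftText convert an incoming string to text and write it to the widget's CenterText and LeftText.
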(event EventBeginPlay
  (bind _returnvalue (UserInterface|CreateWidget "/Game/Learn_Collision/HudWidget.HudWidget_C"))
  (bind _output_get (Variables|Default|SetHudWidget _returnvalue))
  (UserInterface|Viewport|AddtoViewport _output_get 0))

(fn ConstructionScript)

(fn SetText
  (params (NewString :type String))
  (Variables|/Game/Learn_Collision/HudWidget.HudWidget_C|SetCenterText (Variables|Default|GetHudWidget) (Utilities|Text|ToText(String) NewString)))

(fn SetLeftText
  (params (NewString :type String))
  (Variables|/Game/Learn_Collision/HudWidget.HudWidget_C|SetLeftText (Variables|Default|GetHudWidget) (Utilities|Text|ToText(String) NewString)))
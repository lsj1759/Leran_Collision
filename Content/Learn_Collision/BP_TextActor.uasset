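; BP_TextActor is a collision-learning actor with a Cube and a widget component that counts player overlaps.
; When BP_MyCharacter begins overlapping the Cube, it increments Count and writes the number to the ActorWidget's Text.
; End overlap only casts to the character and changes nothing.
; Unconnected nodes that would show begin and end overlap messages never run.
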(event OnComponentEndOverlap(Cube)
  (params (OverlappedComponent :type Primitive%20Component%20Object%20Reference) (OtherActor :type Actor%20Object%20Reference) (OtherComp :type Primitive%20Component%20Object%20Reference) (OtherBodyIndex :type Integer))
  (Utilities|Casting|CastToBP_MyCharacter OtherActor))

(event OnComponentBeginOverlap(Cube)
  (params (OverlappedComponent :type Primitive%20Component%20Object%20Reference) (OtherActor :type Actor%20Object%20Reference) (OtherComp :type Primitive%20Component%20Object%20Reference) (OtherBodyIndex :type Integer) (bFromSweep :type Boolean) (SweepResult :type Hit%20Result%20Structure%20%28by%20ref%29))
  (Utilities|Casting|CastToBP_MyCharacter OtherActor)
  (Math|Integer|IncrementInt (Variables|Default|GetCount)
    (:%20%20
      (bind _asactor_widget (Utilities|Casting|CastToActorWidget (UserInterface|GetUserWidgetObject (Variables|Default|GetWidget))))
      (Variables|/Game/Learn_Collision/ActorWidget.ActorWidget_C|SetText _asactor_widget (Utilities|Text|ToText(Integer) (Variables|Default|GetCount))))))

(event EventBeginPlay)

(fn ConstructionScript)